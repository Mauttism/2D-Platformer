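; Scrap pickup that adds its ScoreUp value to the player's score when touched.
; An overlap on the interactive collider casts to BP_PlayerBase_Adam and rebuilds its Player struct with the increased Score, leaving other fields unchanged.
; PickupConsumed then hides FBInteractive and destroys the collider so it triggers only once, without destroying the actor.
; The new score is printed to screen.
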(event OnComponentBeginOverlap(Interactive_Collider)
  (params (OverlappedComponent :type Primitive%20Component%20Object%20Reference) (OtherActor :type Actor%20Object%20Reference) (OtherComp :type Primitive%20Component%20Object%20Reference) (OtherBodyIndex :type Integer) (bFromSweep :type Boolean) (SweepResult :type Hit%20Result%20Structure%20%28by%20ref%29))
  (bind _asbp_player_base_adam (Utilities|Casting|CastToBP_PlayerBase_Adam OtherActor))
  (bind _output_get (Variables|/Game/Adam/Blueprints/Player/BP_PlayerBase_Adam.BP_PlayerBase_Adam_C|SetPlayer _asbp_player_base_adam (Utilities|Struct|MakeS_PlayerStats_Adam (.default_health (Variables|/Game/Adam/Blueprints/Player/BP_PlayerBase_Adam.BP_PlayerBase_Adam_C|GetPlayer _asbp_player_base_adam)) (.health (Variables|/Game/Adam/Blueprints/Player/BP_PlayerBase_Adam.BP_PlayerBase_Adam_C|GetPlayer _asbp_player_base_adam)) (.default_speed (Variables|/Game/Adam/Blueprints/Player/BP_PlayerBase_Adam.BP_PlayerBase_Adam_C|GetPlayer _asbp_player_base_adam)) (.speed (Variables|/Game/Adam/Blueprints/Player/BP_PlayerBase_Adam.BP_PlayerBase_Adam_C|GetPlayer _asbp_player_base_adam)) (.default_jump_strength (Variables|/Game/Adam/Blueprints/Player/BP_PlayerBase_Adam.BP_PlayerBase_Adam_C|GetPlayer _asbp_player_base_adam)) (.jump_strength (Variables|/Game/Adam/Blueprints/Player/BP_PlayerBase_Adam.BP_PlayerBase_Adam_C|GetPlayer _asbp_player_base_adam)) (.jump_damage (Variables|/Game/Adam/Blueprints/Player/BP_PlayerBase_Adam.BP_PlayerBase_Adam_C|GetPlayer _asbp_player_base_adam)) (.attack_damage (Variables|/Game/Adam/Blueprints/Player/BP_PlayerBase_Adam.BP_PlayerBase_Adam_C|GetPlayer _asbp_player_base_adam)) (.dead (Variables|/Game/Adam/Blueprints/Player/BP_PlayerBase_Adam.BP_PlayerBase_Adam_C|GetPlayer _asbp_player_base_adam)) (+ (.score (Variables|/Game/Adam/Blueprints/Player/BP_PlayerBase_Adam.BP_PlayerBase_Adam_C|GetPlayer _asbp_player_base_adam)) (Variables|Default|GetscoreUp)))))
  (CallFunction|PickupConsumed)
  (Development|PrintString (Utilities|String|ToString(Integer) (.score _output_get))))

(event EventBeginPlay
  (|CallParentFunction) ; This node is disabled and will not be called.\nDrag off pins to build functionality.
)

(fn ConstructionScript
  (|CallParentFunction))

(fn PickupConsumed
  (Rendering|SetVisibility (Variables|Default|GetFB_Interactive) false false)
  (Components|DestroyComponent (Variables|Default|GetInteractive_Collider))
  (return))