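; BP_Jumpbooost is a one-shot pickup that boosts the player's jump.
; When a BP_PlayerBase_Adam overlaps Interactive_Collider, it multiplies that player's JumpMaxHoldTime by JumpMult and prints a message.
; PickupConsumed then hides FBInteractive and destroys the collider, leaving the actor in place.
; Nothing in this Blueprint reverts the boost.
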(event OnComponentBeginOverlap(Interactive_Collider)
  (params (OverlappedComponent :type Primitive%20Component%20Object%20Reference) (OtherActor :type Actor%20Object%20Reference) (OtherComp :type Primitive%20Component%20Object%20Reference) (OtherBodyIndex :type Integer) (bFromSweep :type Boolean) (SweepResult :type Hit%20Result%20Structure%20%28by%20ref%29))
  (bind _asbp_player_base_adam (Utilities|Casting|CastToBP_PlayerBase_Adam OtherActor))
  (Variables|/Script/Engine.Character|SetJumpMaxHoldTime _asbp_player_base_adam (* (Variables|/Script/Engine.Character|GetJumpMaxHoldTime _asbp_player_base_adam) (Variables|Default|GetJump_Mult)))
  (Development|PrintString "Jump Hieght Incressed")
  (CallFunction|PickupConsumed))

(event EventBeginPlay
  (|CallParentFunction) ; This node is disabled and will not be called.\nDrag off pins to build functionality.
)

(fn ConstructionScript
  (|CallParentFunction))

(fn PickupConsumed
  (Rendering|SetVisibility (Variables|Default|GetFB_Interactive) false false)
  (Components|DestroyComponent (Variables|Default|GetInteractive_Collider))
  (return))