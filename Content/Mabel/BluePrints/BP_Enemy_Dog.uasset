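; BP_Enemy_Dog is a side-scrolling dog enemy that walks continuously along the X axis, starting in a random direction.
; Tick feeds constant movement input, and capsule hits with a horizontal normal from anything but the player flip its direction and mirror the sprite via X scale.
; A DoOnce reset after a short delay debounces repeated flips.
; On death it calls the parent handler and destroys itself.
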(event OnComponentHit(CapsuleComponent)
  (params (HitComponent :type Primitive%20Component%20Object%20Reference) (OtherActor :type Actor%20Object%20Reference) (OtherComp :type Primitive%20Component%20Object%20Reference) (NormalImpulse :type Vector :default "0, 0, 0") (Hit :type Hit%20Result%20Structure%20%28by%20ref%29))
  (if (!= OtherActor (Game|Player|GetPlayerPawn 0))
    (if (!= (.X (Math|Vector|BreakVector (.normal Hit))) 0.0)
      (Utilities|FlowControl|DoOnce false
        (:Completed
          (Variables|Default|SetMove_Right (not (Variables|Default|GetMove_Right)))
          (CallFunction|RotateSprite)
          (Utilities|FlowControl|Delay 0.1)
          (CallFunction|ResetDirCheck))))))

(event Custom|ResetDirCheck
  (Utilities|FlowControl|DoOnce false) ; enters at Reset
)

(event EventBeginPlay
  (Variables|Default|SetMove_Right (Math|Random|RandomBool))
  (CallFunction|RotateSprite))

(event Collision|EventActorBeginOverlap
  (params (OtherActor :type Actor%20Object%20Reference)))

(event EventTick
  (params (DeltaSeconds :type Float%20%28single-precision%29))
  (Pawn|Input|AddMovementInput "1.000000, 0, 0" (select (Variables|Default|GetMove_Right) 1.0 -1.0) false))

(fn ConstructionScript
  (|CallParentFunction))

(fn EnemyDied
  (|CallParentFunction)
  (Actor|DestroyActor))

(fn RotateSprite
  (bind _sprite (Variables|Default|GetSprite))
  (bind _returnvalue (Transformation|GetWorldScale _sprite))
  (Transformation|SetWorldScale3D (Variables|Default|GetSprite) (Math|Vector|MakeVector (* (Math|Float|Absolute(Float) (.x _returnvalue)) (select (Variables|Default|GetMove_Right) -1.0 1.0)) (.y _returnvalue) (.z _returnvalue))))