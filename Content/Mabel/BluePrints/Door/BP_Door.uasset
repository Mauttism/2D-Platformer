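; BP_Door is a flipbook-animated door that opens and closes automatically for the player character, BP_PlayerBase_Adam.
; A player hit on the interactive collider opens the door, then after a delay switches its Pawn response to Overlap to allow passage.
; When the player's overlap ends, the door closes and the collider returns to Block after a delay.
; Closing reuses the opening flipbook at a negative play rate, then swaps to the closed flipbook.
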(event OnComponentEndOverlap(Interactive_Collider)
  (params (OverlappedComponent :type Primitive%20Component%20Object%20Reference) (OtherActor :type Actor%20Object%20Reference) (OtherComp :type Primitive%20Component%20Object%20Reference) (OtherBodyIndex :type Integer))
  (Utilities|Casting|CastToBP_PlayerBase_Adam OtherActor)
  (CallFunction|CloseDoor)
  (Utilities|FlowControl|Delay 1.0)
  (Collision|SetCollisionResponsetoChannel (Variables|Default|GetInteractive_Collider) "ECC_Pawn" "ECR_Block"))

(event OnComponentHit(Interactive_Collider)
  (params (HitComponent :type Primitive%20Component%20Object%20Reference) (OtherActor :type Actor%20Object%20Reference) (OtherComp :type Primitive%20Component%20Object%20Reference) (NormalImpulse :type Vector :default "0, 0, 0") (Hit :type Hit%20Result%20Structure%20%28by%20ref%29))
  (Utilities|Casting|CastToBP_PlayerBase_Adam OtherActor)
  (CallFunction|OpenDoor)
  (Utilities|FlowControl|Delay 1.0)
  (Collision|SetCollisionResponsetoChannel (Variables|Default|GetInteractive_Collider) "ECC_Pawn" "ECR_Overlap"))

(event Custom|CloseDoor
  (bind _fb_interactive (Variables|Default|GetFB_Interactive))
  ;[1 1 1] Closes Door
  (Components|Timeline|SetPlayRate _fb_interactive -1.0)
  (Sprite|SetFlipbook _fb_interactive (Variables|Default|GetDoorOpening))
  (Utilities|FlowControl|Delay 1.0)
  (Sprite|SetFlipbook _fb_interactive (Variables|Default|GetDoorClosed)))

(event Custom|OpenDoor
  (bind _fb_interactive (Variables|Default|GetFB_Interactive))
  ;[1 1 1] Opens Door
  (Components|Timeline|SetPlayRate _fb_interactive 1.0)
  (Sprite|SetFlipbook _fb_interactive (Variables|Default|GetDoorOpening))
  (Utilities|FlowControl|Delay 1.0)
  (Sprite|SetFlipbook _fb_interactive (Variables|Default|GetDoorOpen)))

(event EventBeginPlay
  (|CallParentFunction)
  (Sprite|SetFlipbook (Variables|Default|GetFB_Interactive) (Variables|Default|GetDoorClosed)))

(event Collision|EventActorBeginOverlap
  (params (OtherActor :type Actor%20Object%20Reference)))

(event EventTick
  (params (DeltaSeconds :type Float%20%28single-precision%29)))

(fn ConstructionScript
  (|CallParentFunction))