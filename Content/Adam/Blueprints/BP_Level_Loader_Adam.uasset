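; Level-end trigger that saves the player's progress and provides level loading for the platformer.
; When BP_PlayerBase_Adam overlaps the box, it rebuilds the player struct with a small capped health bonus, fixed values and the existing score, saves state, then shows the W_End_Level widget.
; A separate LoadLevel function records LevelName as the game instance's current level before opening it; the overlap does not call it.
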(event OnComponentBeginOverlap(Box)
  (params (OverlappedComponent :type Primitive%20Component%20Object%20Reference) (OtherActor :type Actor%20Object%20Reference) (OtherComp :type Primitive%20Component%20Object%20Reference) (OtherBodyIndex :type Integer) (bFromSweep :type Boolean) (SweepResult :type Hit%20Result%20Structure%20%28by%20ref%29))
  (bind _asbp_player_base_adam (Utilities|Casting|CastToBP_PlayerBase_Adam OtherActor))
  (Variables|/Game/Adam/Blueprints/Player/BP_PlayerBase_Adam.BP_PlayerBase_Adam_C|SetPlayer _asbp_player_base_adam (Utilities|Struct|MakeS_PlayerStats_Adam 8e+01 (Math|Float|Clamp(Float) (+ (.health (Variables|/Game/Adam/Blueprints/Player/BP_PlayerBase_Adam.BP_PlayerBase_Adam_C|GetPlayer _asbp_player_base_adam)) 16.0) 0.0 (.default_health (Variables|/Game/Adam/Blueprints/Player/BP_PlayerBase_Adam.BP_PlayerBase_Adam_C|GetPlayer _asbp_player_base_adam))) 125.0 125.0 1.5e+02 1.5e+02 2e+01 4e+01 false (.score (Variables|/Game/Adam/Blueprints/Player/BP_PlayerBase_Adam.BP_PlayerBase_Adam_C|GetPlayer _asbp_player_base_adam))))
  (Default|SaveState _asbp_player_base_adam false)
  (bind _returnvalue (UserInterface|CreateWidget "/Game/Mabel/BluePrints/W_End_Level.W_End_Level_C"))
  (UserInterface|Viewport|AddtoViewport _returnvalue 1))

(fn ConstructionScript)

(fn LoadLevel
  ;[1 1 1 1 10] This makes sure to set the Current Level in the game instance before opening the level
  (bind _asbp_platformer_game_instance_adam (Utilities|Casting|CastToBP_PlatformerGameInstance_Adam (Game|GetGameInstance)))
  (bind _output_get (Variables|/Game/Adam/Blueprints/BP_PlatformerGameInstance_Adam.BP_PlatformerGameInstance_Adam_C|SetCurrent_Level _asbp_platformer_game_instance_adam (Variables|Default|GetLevel_Name)))
  (Game|OpenLevel(byName) _output_get))