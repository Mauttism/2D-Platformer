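; BP_Spawner_Adam is a one-shot spawner that the player triggers by overlap.
; Either an actor overlap or an Interactive_Collider overlap runs the same logic, which casts the other actor to BP_PlayerBase_Adam and sets an Exhausted flag to block repeats.
; It then spawns the RollerReference class at RelativeSpawnLocation with the player as Instigator, adjusting for collisions but always spawning.
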(event OnComponentBeginOverlap(Interactive_Collider)
  (params (OverlappedComponent :type Primitive%20Component%20Object%20Reference) (OtherActor :type Actor%20Object%20Reference) (OtherComp :type Primitive%20Component%20Object%20Reference) (OtherBodyIndex :type Integer) (bFromSweep :type Boolean) (SweepResult :type Hit%20Result%20Structure%20%28by%20ref%29))
  (if (not (Variables|Default|GetExhausted))
    (bind _asbp_player_base_adam (Utilities|Casting|CastToBP_PlayerBase_Adam (stale Collision|EventActorBeginOverlap OtherActor)))
    (Variables|Default|SetExhausted true)
    (Game|SpawnActorfromClass (Variables|Default|GetRoller_Reference) (Variables|Default|GetRelative%20Spawn%20Location) "AdjustIfPossibleButAlwaysSpawn" 0 _asbp_player_base_adam)))

(event EventBeginPlay
  (|CallParentFunction) ; This node is disabled and will not be called.\nDrag off pins to build functionality.
)

(event Collision|EventActorBeginOverlap
  (params (OtherActor :type Actor%20Object%20Reference))
  (if (not (Variables|Default|GetExhausted))
    (bind _asbp_player_base_adam (Utilities|Casting|CastToBP_PlayerBase_Adam OtherActor))
    (Variables|Default|SetExhausted true)
    (Game|SpawnActorfromClass (Variables|Default|GetRoller_Reference) (Variables|Default|GetRelative%20Spawn%20Location) "AdjustIfPossibleButAlwaysSpawn" 0 _asbp_player_base_adam)))

(event EventTick
  (params (DeltaSeconds :type Float%20%28single-precision%29)))

(fn ConstructionScript
  (|CallParentFunction))