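; Elevator platform that travels vertically between its placed position and a point Range units above when the player hits its interactive collider.
; Construction caches both endpoints, and a timeline lerps the root's world location between them without sweeping.
; On trigger, SetState compares the position to the start with a small tolerance to play forward or reverse, while InMotion blocks retriggering until the move finishes.
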(event OnComponentHit(Interactive_Collider)
  (params (HitComponent :type Primitive%20Component%20Object%20Reference) (OtherActor :type Actor%20Object%20Reference) (OtherComp :type Primitive%20Component%20Object%20Reference) (NormalImpulse :type Vector :default "0, 0, 0") (Hit :type Hit%20Result%20Structure%20%28by%20ref%29))
  (Utilities|Casting|CastToBP_PlayerBase_Adam OtherActor)
  (CallFunction|StartMotion))

(event Custom|Start%20Motion
  (if (not (Variables|Default|GetIn_Motion))
    (CallFunction|SetState)
    (Variables|Default|SetIn_Motion true)
    (switch int (Variables|Default|GetState)
      (:Default
        (bind _float_track (Timeline|Platform%20Timeline ReverseFromEnd)
          (:Update
            (Transformation|SetWorldLocation (Variables|Default|GetDefaultSceneRoot) (Math|Vector|Lerp(Vector) (Variables|Default|GetStart_Location) (Variables|Default|GetEnd%20Location) _float_track) false false))
          (:Finished
            (Variables|Default|SetIn_Motion false))))
      (:0
        (Timeline|Platform%20Timeline PlayFromStart)))))

(event EventBeginPlay
  (|CallParentFunction) ; This node is disabled and will not be called.\nDrag off pins to build functionality.
)

(event Collision|EventActorBeginOverlap
  (params (OtherActor :type Actor%20Object%20Reference)))

(event EventTick
  (params (DeltaSeconds :type Float%20%28single-precision%29)))

(fn ConstructionScript
  (|CallParentFunction)
  (bind _output_get (Variables|Default|SetStart_Location (Transformation|GetWorldLocation (Variables|Default|GetDefaultSceneRoot))))
  (Variables|Default|SetEnd%20Location (Math|Vector|MakeVector (.x _output_get) (.y _output_get) (+ (.z _output_get) (Variables|Default|GetRange))))
  (Variables|Default|SetState 0)
  (Variables|Default|SetIn_Motion false))

(fn SetState
  (if (Math|Vector|Equal(Vector) (Transformation|GetWorldLocation (Variables|Default|GetDefaultSceneRoot)) (Variables|Default|GetStart_Location) 5.0)
    (Variables|Default|SetState 0)
    (else
      (Variables|Default|SetState 1))))