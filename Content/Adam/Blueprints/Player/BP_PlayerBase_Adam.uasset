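; Base 2D platformer player character with run toggle, jump, duck and weapon attack, drawn with Paper2D flipbooks.
; Tick derives a movement state enum to pick the flipbook, turns the player by X velocity and reveals the health bar in game.
; Capsule hit direction decides between stomping enemies and taking damage with knockback.
; The stats struct saves to and restores from the game instance, and death disables the player before opening the death menu.
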(event OnComponentHit(CapsuleComponent)
  (params (HitComponent :type Primitive%20Component%20Object%20Reference) (OtherActor :type Actor%20Object%20Reference) (OtherComp :type Primitive%20Component%20Object%20Reference) (NormalImpulse :type Vector :default "0, 0, 0") (Hit :type Hit%20Result%20Structure%20%28by%20ref%29))
  (bind _self self)
  (bind _charactermovement (Variables|Character|GetCharacterMovement))
  (bind _charactermovement_2 (Variables|Character|GetCharacterMovement))
  ;[1 1 1 1 10] Creates reference to enemy that has been hit
  (bind _asbp_base_enemy_adam (Utilities|Casting|CastToBP_BaseEnemy_Adam OtherActor))
  (Variables|Default|SetHit_Enemy_ref _asbp_base_enemy_adam)
  ;[1 1 1 1 10] Creates reference to hit direction
  (bind _output_get (Variables|Default|SetHitDirection (Math|Vector|Normalize (- (.location Hit) (Transformation|GetActorLocation)) 0.0)))
  (Development|PrintString (Utilities|String|ToString(Float) (.z _output_get)) true true "(R=0.000000,G=0.660000,B=1.000000,A=1.000000)" 1e+01)
  (if (<= (.z (Variables|Default|GetHitDirection)) -0.9)
    (Development|PrintString "Hit" true true "(R=0.000000,G=1.000000,B=0.206126,A=1.000000)" 1e+01)
    ;[1 1 1 1 10] Uses Character Movement component to stop movement immediately, then add a velocity direction
    (Variables|/Script/Engine.MovementComponent|SetVelocity _charactermovement "0, 0, 0")
    (Components|Movement|StopMovementImmediately _charactermovement)
    (Physics|AddImpulse _charactermovement "0, 0,200.000000" true)
    ;[1 1 1] Player damaging enemy class
    (Game|Damage|ApplyDamage (Variables|Default|GetHit_Enemy_ref) (.jump_damage (Variables|Default|GetPlayer self)) 0 0)
    (else
      (Development|PrintString "Got hit" true true "(R=1.000000,G=0.000000,B=0.034835,A=1.000000)" 1e+01)
      ;[1 1 1 1 10] Uses Character Movement component to stop movement immediately, then add a velocity direction
      (Variables|/Script/Engine.MovementComponent|SetVelocity _charactermovement_2 "0, 0, 0")
      (Components|Movement|StopMovementImmediately _charactermovement_2)
      (Physics|AddImpulse _charactermovement_2 (Math|Vector|MakeVector (* (.x (Variables|Default|GetHitDirection)) (* -1.0 (.horizontal_knockback (Variables|/Game/Adam/Blueprints/Enemies/BP_BaseEnemy_Adam.BP_BaseEnemy_Adam_C|GetStats (Variables|Default|GetHit_Enemy_ref))))) 0.0 (.vertical_knockback (Variables|/Game/Adam/Blueprints/Enemies/BP_BaseEnemy_Adam.BP_BaseEnemy_Adam_C|GetStats (Variables|Default|GetHit_Enemy_ref)))) true)
      ;[1 1 1] Enemy class damaging player
      (if (not (.dead (Variables|Default|GetPlayer _self)))
        (Game|Damage|ApplyDamage _self (.damage (Variables|/Game/Adam/Blueprints/Enemies/BP_BaseEnemy_Adam.BP_BaseEnemy_Adam_C|GetStats (Variables|Default|GetHit_Enemy_ref))) 0 0)
        (Development|PrintString (Utilities|String|ToString(Float) (.damage (Variables|/Game/Adam/Blueprints/Enemies/BP_BaseEnemy_Adam.BP_BaseEnemy_Adam_C|GetStats (Variables|Default|GetHit_Enemy_ref)))))))))

(event OnComponentHit(Player_Weapon)
  (params (HitComponent :type Primitive%20Component%20Object%20Reference) (OtherActor :type Actor%20Object%20Reference) (OtherComp :type Primitive%20Component%20Object%20Reference) (NormalImpulse :type Vector :default "0, 0, 0") (Hit :type Hit%20Result%20Structure%20%28by%20ref%29))
  ;[0 0.04274 1 1 16] Handles updating player health
  ;;[1 1 1] Player Attack Collision
  (bind _asbp_base_enemy_adam (Utilities|Casting|CastToBP_BaseEnemy_Adam OtherActor))
  (if (Variables|Default|GetAttacking)
    (Game|Damage|ApplyDamage _asbp_base_enemy_adam (.attack_damage (Variables|Default|GetPlayer)) 0 0)
    (Development|PrintString "Enemy Struck")))

(event Game|Damage|EventAnyDamage
  (params (Damage :type Float%20%28single-precision%29) (DamageType :type Damage%20Type%20Object%20Reference) (InstigatedBy :type Controller%20Object%20Reference) (DamageCauser :type Actor%20Object%20Reference))
  ;[0 0.04274 1 1 16] Handles updating player health
  (bind _output_get (Variables|Default|SetPlayer (Utilities|Struct|MakeS_PlayerStats_Adam (.default_health (Variables|Default|GetPlayer)) (Math|Float|Clamp(Float) (- (.health (Variables|Default|GetPlayer)) Damage) 0.0 (.default_health (Variables|Default|GetPlayer))) (.default_speed (Variables|Default|GetPlayer)) (.speed (Variables|Default|GetPlayer)) (.default_jump_strength (Variables|Default|GetPlayer)) (.jump_strength (Variables|Default|GetPlayer)) (.jump_damage (Variables|Default|GetPlayer)) (.attack_damage (Variables|Default|GetPlayer)) (.dead (Variables|Default|GetPlayer)) (.score (Variables|Default|GetPlayer)))))
  (CallFunction|UpdateHealthBar)
  ;;[1 1 1 1 20] Makes sure the health is less than or equal to zero, and that the player has not died already
  (if (and (<= (.health _output_get) 0.0) (not (.dead _output_get)))
    (Variables|Default|SetPlayer (Utilities|Struct|MakeS_PlayerStats_Adam (.default_health _output_get) (.health _output_get) (.default_speed _output_get) (.speed _output_get) (.default_jump_strength _output_get) (.jump_strength _output_get) (.jump_damage _output_get) (.attack_damage _output_get) true (.score _output_get)))
    ;;[1 0.9926 0.9705] Sets animations and colliders
    (CallFunction|PlayerDied)
    (Utilities|FlowControl|Delay 1.0)
    ;;[0.06837 1 0] Here lies where the player died widget shall be created and added to viewport.
    (bind _returnvalue (UserInterface|CreateWidget "/Game/Adam/Blueprints/UI/WBP_Death_Menu.WBP_Death_Menu_C"))
    (UserInterface|Viewport|AddtoViewport _returnvalue 4)))

(event EventBeginPlay
  (Variables|Default|SetMovementState "NewEnumerator6")
  (CallFunction|RestoreState)
  (bind _returnvalue (UserInterface|CreateWidget "/Game/Adam/Blueprints/UI/WBP_PlayerHealth_Adam.WBP_PlayerHealth_Adam_C"))
  (bind _output_get (Variables|Default|SetHealth_Bar_ref _returnvalue))
  (UserInterface|Viewport|AddtoViewport _output_get 0)
  (CallFunction|UpdateHealthBar)
  (bind _in_game (CallFunction|CheckinGame))
  (if _in_game
    (Widget|SetVisibility (Variables|Default|GetHealth_Bar_ref) "Visible")
    (else
      (Widget|SetVisibility (Variables|Default|GetHealth_Bar_ref) "Collapsed"))))

(event EventTick
  (params (DeltaSeconds :type Float%20%28single-precision%29))
  (Utilities|FlowControl|Sequence
    (:then_0
      ;[0.9767 0.9897 1 1 10] These functions both maintain the player sprite so it corresponds to the proper input
      (CallFunction|UpdateFlipbook))
    (:then_1
      (CallFunction|UpdatePlayerRotation))
    (:then_2
      ;[1 1 1] This function hides any persistant UI until a level is loaded
      (CallFunction|UpdateUI))))

(event Input|KeyboardEvents|H
  (params (Key :type Key%20Structure))
  ;[1 0 0] Debug
  (:Pressed
    (Game|Damage|ApplyDamage self 4.0 0 0)))

(event Input|ActionEvents|InputActionAttack
  (params (Key :type Key%20Structure))
  ;[1 1 1] Attack Input
  (:Pressed
    (CallFunction|ValidateAttack)
    ;;[1 1 1] If player is "Attacking" The weapon capsule is moved out
    (CallFunction|Attack (Variables|Default|GetAttacking))
    ;;[1 1 1 1 10] Set to .45 rather than .5 because .5 clips the begining frame of the animation
    (Utilities|FlowControl|Delay 0.45 :!label _label)
    (Variables|Default|SetAttacking false))
  (:Released
    (goto _label)))

(event Input|ActionEvents|InputActionJump
  (params (Key :type Key%20Structure))
  ;[1 1 1] Handles Jump Input
  (:Pressed
    (Character|Jump))
  (:Released
    (Character|StopJumping)))

(event Input|ActionEvents|InputActionDuck
  (params (Key :type Key%20Structure))
  ;[1 1 1] Sets Ducking variable, and changes the half height, and walk speed
  (:Pressed
    (Transformation|SetRelativeLocation (Variables|Default|GetSpringArm) "0, 0,4.000000" true false)
    (Variables|Default|SetDucking true)
    (Components|Capsule|SetCapsuleHalfHeight (Variables|Collision|GetCapsuleComponent) 1e+01 true)
    (Variables|/Script/Engine.CharacterMovementComponent|SetMaxWalkSpeed (Variables|Character|GetCharacterMovement) 0.0))
  (:Released
    (Transformation|SetRelativeLocation (Variables|Default|GetSpringArm) "0, 0, 0" true false)
    (Variables|Default|SetDucking false)
    (Components|Capsule|SetCapsuleHalfHeight (Variables|Collision|GetCapsuleComponent) 14.0 true)
    (CallFunction|ToggleSpeed (Variables|Default|GetSprinting))))

(event Input|ActionEvents|InputActionToggle_Run
  (params (Key :type Key%20Structure))
  ;[1 1 1] Toggle Run/Walk Input
  (:Pressed
    (bind _sprinting (CallFunction|ToggleSprinting))
    (CallFunction|ToggleSpeed _sprinting)))

(event Input|AxisEvents|InputAxisMoveRight
  (params (AxisValue :type Float%20%28single-precision%29))
  ;[1 1 1] Handles Left and Right movement
  (Pawn|Input|AddMovementInput "1.000000, 0,0.000000" AxisValue false))

(fn ConstructionScript
  (bind _charactermovement (Variables|Character|GetCharacterMovement))
  (bind _output_get (Variables|Default|SetPlayer (Utilities|Struct|MakeS_PlayerStats_Adam 8e+01 8e+01 125.0 125.0 1.5e+02 1.5e+02 2e+01 4e+01 false 0)))
  (Variables|/Script/Engine.CharacterMovementComponent|SetMaxWalkSpeed _charactermovement (.default_speed _output_get))
  (Variables|/Script/Engine.CharacterMovementComponent|SetJumpZVelocity _charactermovement (.default_jump_strength _output_get))
  (CallFunction|SaveState true))

(fn UpdateFlipbook
  (bind _output (CallFunction|GetFlipbookEnum)) ; This Function finds the movement state of the player
  (bind _output_get (Variables|Default|SetMovementState _output))
  (Sprite|SetFlipbook (Variables|Default|GetSprite) (Utilities|Select :Index _output_get :NewEnumerator6 0 :NewEnumerator4 (Variables|Default|GetFB_Idle) :NewEnumerator0 (Variables|Default|GetFB_Run) :NewEnumerator1 (Variables|Default|GetFB_Jump) :NewEnumerator2 (Variables|Default|GetFB_Fall) :NewEnumerator3 (Variables|Default|GetFB_Duck) :NewEnumerator5 (Variables|Default|GetFB_Attack) :NewEnumerator7 (Variables|Default|GetFB_Fall_Attack) :NewEnumerator8 (Variables|Default|GetFB_Duck_Attack))))

(fn UpdatePlayerRotation
  ;[1 1 1] Uses x velocity to decide yaw of Player Controller
  (Math|Float|CompareFloat (.x (Transformation|GetVelocity)) 0.0
    (:>
      (Pawn|SetControlRotation (Game|GetPlayerController 0) (Math|Rotator|MakeRotator 0.0 0.0 0.0)))
    (:<
      (Pawn|SetControlRotation (Game|GetPlayerController 0) (Math|Rotator|MakeRotator 0.0 0.0 1.8e+02)))))

(fn GetFlipbookEnum
  (bind _output_get (Variables|Default|SetMovementState (select (AI|Components|NavMovement|IsFalling (Variables|Character|GetCharacterMovement)) (select (<= (.z (Transformation|GetVelocity)) 0.0) (select (Variables|Default|GetAttacking) "NewEnumerator7" "NewEnumerator2") "NewEnumerator1") (select (!= (Math|Vector|VectorLength (Transformation|GetVelocity)) 0.0) (select (Variables|Default|GetAttacking) "NewEnumerator5" "NewEnumerator0") (select (and (Variables|Default|GetDucking) (Variables|Default|GetAttacking)) "NewEnumerator8" (select (Variables|Default|GetDucking) "NewEnumerator3" (select (Variables|Default|GetAttacking) "NewEnumerator5" "NewEnumerator4")))))))
  (return _output_get))

(fn PlayerDied
  (bind _effects (Variables|Default|GetEffects))
  (bind _charactermovement (Variables|Character|GetCharacterMovement))
  (CallFunction|SaveState false)
  (Variables|Default|SetPlayer (Utilities|Struct|MakeS_PlayerStats_Adam 8e+01 8e+01 125.0 125.0 1.5e+02 1.5e+02 2e+01 4e+01 true 0))
  (Input|DisableInput (Game|GetPlayerController 0))
  (Rendering|SetVisibility (Variables|Default|GetSprite) false false)
  (Rendering|SetVisibility _effects true false)
  (Components|Timeline|SetLooping _effects false)
  (Collision|SetCollisionEnabled (Variables|Collision|GetCapsuleComponent) "NoCollision")
  (Variables|/Script/Engine.CharacterMovementComponent|SetGravityScale _charactermovement 0.0)
  (Pawn|Components|CharacterMovement|DisableMovement _charactermovement))

(fn UpdateHealthBar
  (bind _player (Variables|Default|GetPlayer))
  (Default|UpdateHealth (Variables|Default|GetHealth_Bar_ref) (.health _player) (.default_health _player)))

(fn SaveState
  (params (Is_Constructor :type Boolean))
  (bind _asbp_platformer_game_instance_adam (Utilities|Casting|CastToBP_PlatformerGameInstance_Adam (Game|GetGameInstance)))
  (Default|SavePlayerInfo _asbp_platformer_game_instance_adam (Variables|Default|GetPlayer) Is_Constructor))

(fn RestoreState
  (bind _asbp_platformer_game_instance_adam (Utilities|Casting|CastToBP_PlatformerGameInstance_Adam (Game|GetGameInstance)))
  (bind _player (Default|RestorePlayerInfo _asbp_platformer_game_instance_adam))
  (Variables|Default|SetPlayer _player))

(fn Attack
  (params (Attacking :type Boolean))
  (bind _player_weapon (Variables|Default|GetPlayer_Weapon))
  (if Attacking
    (Transformation|SetRelativeLocation _player_weapon "12.000000, 0,6.000000" true false)
    (else
      (Transformation|SetRelativeLocation _player_weapon "0, 0,6.000000" false true))))

(fn CheckinGame
  (bind _asbp_platformer_game_instance_adam (Utilities|Casting|CastToBP_PlatformerGameInstance_Adam (Game|GetGameInstance)))
  (return (Variables|/Game/Adam/Blueprints/BP_PlatformerGameInstance_Adam.BP_PlatformerGameInstance_Adam_C|GetIn_Game _asbp_platformer_game_instance_adam)))

(fn UpdateUI
  (bind _in_game (CallFunction|CheckinGame))
  (if _in_game
    (Utilities|FlowControl|DoOnce false :!label _label
      (:Completed
        (Widget|SetVisibility (Variables|Default|GetHealth_Bar_ref) "Visible")))
    (else
      (goto _label Reset))))

(fn ToggleSprinting
  (bind _output_get (Variables|Default|SetSprinting (not (Variables|Default|GetSprinting))))
  (return _output_get))

(fn ToggleSpeed
  (params (Condition :type Boolean))
  (bind _player (Variables|Default|GetPlayer))
  (bind _charactermovement (Variables|Character|GetCharacterMovement))
  (if Condition
    (Variables|/Script/Engine.CharacterMovementComponent|SetMaxWalkSpeed _charactermovement (.speed _player))
    (Components|Timeline|SetPlayRate (Variables|Default|GetSprite) 1.0)
    (else
      (Variables|/Script/Engine.CharacterMovementComponent|SetMaxWalkSpeed _charactermovement (/ (.speed _player) 2.0))
      (Components|Timeline|SetPlayRate (Variables|Default|GetSprite) 0.75))))

(fn ValidateAttack
  (bind _charactermovement (Variables|Character|GetCharacterMovement))
  (bind _velocity (Variables|/Script/Engine.MovementComponent|GetVelocity _charactermovement))
  (Variables|Default|SetAttacking (or (Math|Boolean|NANDBoolean (> (Math|Float|Absolute(Float) (.x _velocity)) 0.0) (== (.z _velocity) 0.0)) (== (.x _velocity) 0.0)))
  (return false))

(fn ResetPlayer
  (bind _effects (Variables|Default|GetEffects))
  (bind _charactermovement (Variables|Character|GetCharacterMovement))
  (Variables|Default|SetPlayer (Utilities|Struct|MakeS_PlayerStats_Adam (.default_health (Variables|Default|GetPlayer)) (.default_health (Variables|Default|GetPlayer)) (.default_speed (Variables|Default|GetPlayer)) (.default_speed (Variables|Default|GetPlayer)) (.default_jump_strength (Variables|Default|GetPlayer)) (.default_jump_strength (Variables|Default|GetPlayer)) (.jump_damage (Variables|Default|GetPlayer)) (.attack_damage (Variables|Default|GetPlayer)) false (- (.score (Variables|Default|GetPlayer)) 1000)))
  (Input|EnableInput (Game|GetPlayerController 0))
  (Rendering|SetVisibility (Variables|Default|GetSprite) true false)
  (Rendering|SetVisibility _effects false false)
  (Components|Timeline|SetLooping _effects true)
  (Collision|SetCollisionEnabled (Variables|Collision|GetCapsuleComponent) "QueryAndPhysics")
  (Variables|/Script/Engine.CharacterMovementComponent|SetGravityScale _charactermovement 1.0)
  (Pawn|Components|CharacterMovement|SetMovementMode _charactermovement "MOVE_Walking" 0)
  (CallFunction|SaveState false))