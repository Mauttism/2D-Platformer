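; Base 2D side-scrolling player character that runs, jumps and crouches with flipbook animation.
; Tick picks the jump, fall, run, crouch or idle flipbook from movement state and velocity, so run overrides crouch while moving.
; It also turns the controller yaw to face the horizontal travel direction.
; Input drives movement along world X, and crouching manually shrinks the capsule and lowers walk speed.
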(event EventTick
  (params (DeltaSeconds :type Float%20%28single-precision%29))
  (Utilities|FlowControl|Sequence
    (:then_0
      ;[1 1 1] Movement Branches, uses input to decide which flip books to use
      (if (AI|Components|NavMovement|IsFalling (Variables|Character|GetCharacterMovement))
        (Sprite|SetFlipbook (Variables|Default|GetSprite) (select (<= (.z (Transformation|GetVelocity)) 0.0) (Variables|Default|GetFB_Fall) (Variables|Default|GetFB_Jump)))
        (elif (!= (Math|Vector|VectorLength (Transformation|GetVelocity)) 0.0)
          (Sprite|SetFlipbook (Variables|Default|GetSprite) (Variables|Default|GetFB_Run))
          (elif (Variables|Default|GetCrouching)
            (Sprite|SetFlipbook (Variables|Default|GetSprite) (Variables|Default|GetFB_Crouch))
            (else
              (Sprite|SetFlipbook (Variables|Default|GetSprite) (Variables|Default|GetFB_Idle)))))))
    (:then_1
      (Math|Float|CompareFloat (.x (Transformation|GetVelocity)) 0.0
        (:>
          (Pawn|SetControlRotation (Game|GetPlayerController 0) (Math|Rotator|MakeRotator 0.0 0.0 0.0)))
        (:<
          (Pawn|SetControlRotation (Game|GetPlayerController 0) (Math|Rotator|MakeRotator 0.0 0.0 1.8e+02)))))))

(event Input|ActionEvents|InputActionCrouch
  (params (Key :type Key%20Structure :default "None"))
  ;[1 1 1] Sets crouching
  (:Pressed
    (Variables|Default|SetCrouching true)
    (Components|Capsule|SetCapsuleHalfHeight (Variables|Collision|GetCapsuleComponent) 12.0 true)
    (Variables|/Script/Engine.CharacterMovementComponent|SetMaxWalkSpeed (Variables|Character|GetCharacterMovement) 75.0))
  (:Released
    (Variables|Default|SetCrouching false)
    (Components|Capsule|SetCapsuleHalfHeight (Variables|Collision|GetCapsuleComponent) 16.0 true)
    (Variables|/Script/Engine.CharacterMovementComponent|SetMaxWalkSpeed (Variables|Character|GetCharacterMovement) 125.0)))

(event Input|ActionEvents|InputActionJump
  (params (Key :type Key%20Structure :default "None"))
  ;[1 1 1] Handles Jump Input
  (:Pressed
    (Character|Jump))
  (:Released
    (Character|StopJumping)))

(event Input|AxisEvents|InputAxisMoveRight
  (params (AxisValue :type Float%20%28single-precision%29))
  ;[1 1 1] Handles Left and Right movement
  (Pawn|Input|AddMovementInput "1.000000, 0, 0" AxisValue false))

(fn ConstructionScript)