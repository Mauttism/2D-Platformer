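; BP_Enemy_Rollers is a 2D flipbook enemy that moves continuously along the X axis, starting in a random direction.
; Capsule hits with an X normal, except from the player, reverse movement and mirror the sprite via X scale, with a DoOnce and short delay debouncing repeated flips.
; It sets its own Stats at construction and extends the parent's death logic with a one-shot explosion flipbook, hiding the sprite and destroying the capsule.
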(event OnComponentHit(CapsuleComponent)
  (params (HitComponent :type Primitive%20Component%20Object%20Reference) (OtherActor :type Actor%20Object%20Reference) (OtherComp :type Primitive%20Component%20Object%20Reference) (NormalImpulse :type Vector :default "0, 0, 0") (Hit :type Hit%20Result%20Structure%20%28by%20ref%29))
  (if (!= OtherActor (Game|Player|GetPlayerPawn 0))
    (if (!= (.X (Math|Vector|BreakVector (.normal Hit))) 0.0)
      (Utilities|FlowControl|DoOnce false
        (:Completed
          (Variables|Default|Setmove_right (not (Variables|Default|Getmove_right)))
          (CallFunction|UpdateFlipbookDirection)
          (Utilities|FlowControl|Delay 0.1)
          (CallFunction|ResetDirectionChangeCheck))))))

(event Custom|Reset_Direction_Change_Check
  (Utilities|FlowControl|DoOnce false) ; enters at Reset
)

(event EventBeginPlay
  (|CallParentFunction)
  (Variables|Default|Setmove_right (Math|Random|RandomBool)))

(event Collision|EventActorBeginOverlap
  (params (OtherActor :type Actor%20Object%20Reference))
  (|CallParentFunction OtherActor) ; This node is disabled and will not be called.\nDrag off pins to build functionality.
)

(event EventTick
  (params (DeltaSeconds :type Float%20%28single-precision%29))
  (|CallParentFunction DeltaSeconds)
  (Pawn|Input|AddMovementInput "1.000000, 0, 0" (select (Variables|Default|Getmove_right) 1.0 -1.0) false))

(fn ConstructionScript
  (|CallParentFunction)
  (Variables|Default|SetStats (Utilities|Struct|MakeS_BaseEnemy 4e+01 4e+01 1e+02 1e+02 4.0 1.5e+02 false)))

(fn EnemyDied
  (bind _fb_effects (Variables|Default|GetFB_Effects))
  (|CallParentFunction)
  (Components|Timeline|SetLooping _fb_effects false)
  (Sprite|SetFlipbook _fb_effects "/Game/Adam/Assets/FB_Explosion.FB_Explosion")
  (Rendering|SetVisibility (Variables|Default|GetSprite) false false)
  (Components|DestroyComponent (Variables|Default|GetCapsuleComponent)))

(fn UpdateFlipbookDirection
  (bind _sprite (Variables|Default|GetSprite))
  (bind _returnvalue (Transformation|GetWorldScale _sprite))
  (Transformation|SetWorldScale3D _sprite (Math|Vector|MakeVector (* (Math|Float|Absolute(Float) (.x _returnvalue)) (select (Variables|Default|Getmove_right) 1.0 -1.0)) (.y _returnvalue) (.z _returnvalue))))