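; BP_Enemy_Drones is a flying 2D flipbook enemy that patrols horizontally around its spawn point, starting in a random direction.
; Tick applies movement input, mirrors the sprite and effects, and reverses direction beyond half of MovementRange from the start.
; Non-player hits with a horizontal normal also reverse it; DoOnce gates prevent repeated flipping.
; Construction sets stats and fly speed, while death plays a one-shot explosion and removes collision.
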(event OnComponentHit(CapsuleComponent)
  (params (HitComponent :type Primitive%20Component%20Object%20Reference) (OtherActor :type Actor%20Object%20Reference) (OtherComp :type Primitive%20Component%20Object%20Reference) (NormalImpulse :type Vector :default "0, 0, 0") (Hit :type Hit%20Result%20Structure%20%28by%20ref%29))
  (if (!= OtherActor (Game|Player|GetPlayerPawn 0))
    (if (!= (.X (Math|Vector|BreakVector (.normal Hit))) 0.0)
      (Utilities|FlowControl|DoOnce false
        (:Completed
          (Variables|Default|Setmove_right (not (Variables|Default|Getmove_right)))
          (CallFunction|UpdateFlipbookDirection)
          (Utilities|FlowControl|Delay 0.1)
          (CallFunction|ResetDirectionChangeCheck))))))

(event Custom|Reset_Direction_Change_Check
  (Utilities|FlowControl|DoOnce false) ; enters at Reset
)

(event EventBeginPlay
  (|CallParentFunction)
  ;[1 1 1 1 12] Gives the drone a 1/2 chancc of starting facing left or right
  (CallFunction|SetStartingDirection))

(event EventTick
  (params (DeltaSeconds :type Float%20%28single-precision%29))
  (|CallParentFunction DeltaSeconds)
  ;[1 1 1 1 12] Gets move right, and sets velocity based on it
  (CallFunction|SetCurrentDirection)
  (CallFunction|UpdateFlipbookDirection)
  ;[1 1 1 1 12] Checks if Drone has exited it's permissable range
  (bind _outside_range (CallFunction|CheckDistance))
  (if _outside_range
    ;[1 1 1 1 12] I wanted to collapse this into a function, but it kept turning into beyblades again
    ;;[1 1 1 1 10] Might be a bad solution, but stops the drones from turning into beyblades
    (Utilities|FlowControl|DoOnce true :!label _label
      (:Completed
        (Variables|Default|Setmove_right (not (Variables|Default|Getmove_right)))))
    (else
      (goto _label Reset))))

(fn ConstructionScript
  (|CallParentFunction)
  (bind _output_get (Variables|Default|SetStats (Utilities|Struct|MakeS_BaseEnemy 2e+01 2e+01 12.5 25.0 16.0 1e+02 1e+02 false)))
  (Variables|/Script/Engine.CharacterMovementComponent|SetMaxFlySpeed (Variables|Character|GetCharacterMovement) (.speed _output_get))
  (Variables|Default|SetMovement_Range 1e+02))

(fn UpdateFlipbookDirection
  (bind _move_right (Variables|Default|Getmove_right))
  (bind _sprite (Variables|Default|GetSprite))
  (bind _returnvalue (Transformation|GetWorldScale _sprite))
  (bind _returnvalue_2 (select _move_right 1.0 -1.0))
  (bind _returnvalue_3 (Math|Float|Absolute(Float) (.x _returnvalue)))
  (bind _returnvalue_4 (* _returnvalue_3 _returnvalue_2))
  (Transformation|SetWorldScale3D _sprite (Math|Vector|MakeVector _returnvalue_4 (.y _returnvalue) (.z _returnvalue)))
  (Transformation|SetWorldScale3D (Variables|Default|GetFB_Effects) (Math|Vector|MakeVector _returnvalue_4 (.y _returnvalue) (.z _returnvalue))))

(fn EnemyDied
  (bind _fb_effects (Variables|Default|GetFB_Effects))
  (|CallParentFunction)
  (Components|Timeline|SetLooping _fb_effects false)
  (Sprite|SetFlipbook _fb_effects "/Game/Adam/Assets/Flipbooks/Effects/FB_Explosion.FB_Explosion")
  (Rendering|SetVisibility (Variables|Default|GetSprite) false false)
  (Components|DestroyComponent (Variables|Default|GetCapsuleComponent)))

(fn CheckDistance
  (return (> (Math|Float|Absolute(Float) (- (.x (Transformation|GetActorLocation)) (.x (Variables|Default|GetStart_Location)))) (/ (Variables|Default|GetMovement_Range) 2.0))))

(fn SetStartingDirection
  (Variables|Default|Setmove_right (Math|Random|RandomBool))
  (Variables|Default|SetStart_Location (Transformation|GetActorLocation self)))

(fn SetCurrentDirection
  (Pawn|Input|AddMovementInput "1.000000, 0, 0" (select (Variables|Default|Getmove_right) 1.0 -1.0) false))