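; Base enemy Blueprint that holds a stats struct and handles damage and death, intended as a parent for specific enemy types.
; The construction script fills health to its default, with a disconnected example showing how children set their own stats.
; AnyDamage subtracts clamped health and, at zero, sets the Dead flag once and calls EnemyDied.
; EnemyDied and GetEffectState are empty, with an unconnected example death that plays an explosion flipbook, hides the sprite and removes collision.
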(event Game|Damage|EventAnyDamage
  (params (Damage :type Float%20%28single-precision%29) (DamageType :type Damage%20Type%20Object%20Reference) (InstigatedBy :type Controller%20Object%20Reference) (DamageCauser :type Actor%20Object%20Reference))
  (bind _output_get (Variables|Default|SetStats (Utilities|Struct|MakeS_BaseEnemy (.default_health (Variables|Default|GetStats)) (Math|Float|Clamp(Float) (- (.health (Variables|Default|GetStats)) Damage) 0.0 (.default_health (Variables|Default|GetStats))) 1e+02 1e+02 8.0 1e+02 (.dead (Variables|Default|GetStats)))))
  ;[1 1 1 1 10] Makes sure the health is less than or equal to zero, and that the enemy has not died already
  (if (and (<= (.health _output_get) 0.0) (not (.dead _output_get)))
    (Variables|Default|SetStats (Utilities|Struct|MakeS_BaseEnemy (.default_health _output_get) (.health _output_get) 1e+02 1e+02 8.0 1e+02 true))
    ;[1 0 0] Debug
    (CallFunction|EnemyDied)))

(fn ConstructionScript
  (Variables|Default|SetStats (Utilities|Struct|MakeS_BaseEnemy (.default_health (Variables|Default|GetStats)) (.default_health (Variables|Default|GetStats)) 1e+02 1e+02 8.0 1e+02 (.dead (Variables|Default|GetStats)))))

(fn EnemyDied)

(fn GetEffectState)